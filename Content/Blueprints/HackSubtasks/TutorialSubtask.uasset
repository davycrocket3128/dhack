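; TutorialSubtask is a hack subtask that shows a tutorial prompt with a configurable title and text.
; On each tick it waits until no tutorial is active, then activates its prompt through the Peacenet tutorial state and sets a shown flag.
; Once that flag is set and no tutorial is active, the subtask finishes.
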(event `self.OnTick`
  (params (InDeltaSeconds :type "Float (single-precision)"))
  (bind _returnvalue (`UserContext.GetPeacenet` (`self.GetPlayerUser`)))
  ;[1 1 1] Is a tutorial currently active?
  (if (not (`PeacenetWorldStateActor.IsTutorialActive` _returnvalue))
    ;[1 1 1] If a tutorial isn't active and we haven't shown our tutorial yet then we show our tutorial.  If we have shown our tutorial, then we finish.
    (if (`self.Has Shown Tutorial`)
      (`self.Finish`)
      (else
        (`TutorialPromptState.ActivatePrompt` (`PeacenetWorldStateActor.GetTutorialState` _returnvalue) (`self.Tutorial Title`) (`self.Tutorial Text`))
        (set `self.Has Shown Tutorial` true)))))