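; Background music component that switches between 2D tracks with a crossfade.
; PlaySound skips a request matching the current track's sound, otherwise spawns a persistent audio component, fades it in and fades out any playing track.
; AboutToPlayNewTrack waits out the fade, destroys the old component and makes the new one current.
; Looping comes from replaying the current track whenever its OnAudioFinished event fires.
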(event `About To Play New Track`
  (params (`Time To Play` :type "Float (double-precision)") (Track :type "AudioComponent Object Reference"))
  (bind _current_audio (`self.Current Audio`))
  ;[1 1 1] Wait for the current track to fade out, then destroy the current track and set the new track as the current track.
  (`KismetSystemLibrary.Delay` `Time To Play`)
  (if (`KismetSystemLibrary.IsValid` _current_audio)
    (clear `AudioComponent.OnAudioFinished` _current_audio)
    (`AudioComponent.Stop` _current_audio)
    (`self.K2_DestroyComponent` _current_audio))
  (bind _output_get (set `self.Current Audio` Track))
  ;[1 1 1] Allow the audio to loop.
  (add `AudioComponent.OnAudioFinished` _output_get (delegate `Loop audio`)))

(event `Loop audio`
  ;[1 1 1] Allow the audio to loop.
  (`AudioComponent.Play` (`self.Current Audio`) 0.0))

(fn `Play Sound`
  (params (Sound :type "SoundBase Object Reference"))
  (bind _current_audio (`self.Current Audio`))
  (bind _current_audio_2 (`self.Current Audio`))
  ;[1 1 1] Skip fade to next track if the next track will end up being the exact same track.
  (if (`KismetSystemLibrary.IsValid` _current_audio_2)
    (if (not (== (`AudioComponent.Sound` _current_audio_2) Sound))
      ;[1 1 1] Create the new sound effect and play it.
      (bind _returnvalue (`GameplayStatics.CreateSound2D` Sound 1.0 1.0 0.0 null false false :!label _label))
      (`AudioComponent.Play` _returnvalue 0.0)
      (`AudioComponent.AdjustVolume` _returnvalue 0.0 0.0)
      (`AudioComponent.AdjustVolume` _returnvalue 2.0 1.0)
      ;[1 1 1] Are we currently playing audio?
      (if (`KismetSystemLibrary.IsValid` _current_audio)
        (if (`AudioComponent.IsPlaying` _current_audio)
          ;[1 1 1] Fade out previous track
          (`AudioComponent.AdjustVolume` _current_audio 2.0 0.0)
          (`self.About To Play New Track` 2.0 _returnvalue)
          (else
            (`self.About To Play New Track` 0.0 _returnvalue :!label _label_2)))
        (else
          (goto _label_2))))
    (else
      (goto _label))))