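; Player pawn for a Peacenet game session, hosting the Peacegate desktop and returning to the menu on quit.
; BeginPlay starts the game, then the system-ready event adds the desktop to the viewport, possesses the pawn and focuses input.
; Input actions open a terminal or toggle text mode.
; Quit requests unpossess the pawn, which removes the desktop, spawns a menu pawn and destroys itself and Peacenet, forcing a save.
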(event `self.ReceiveBeginPlay`
  (bind _peacenet (`self.Peacenet`))
  ;[1 1 1] Start the game.
  (add `PeacenetWorldStateActor.PlayerSystemReady` _peacenet (delegate `Player System Ready`))
  (`PeacenetWorldStateActor.StartGame` _peacenet "/Game/UserInterface/Desktop/Desktop.Desktop_C" "/Game/UserInterface/Widgets/WindowBorder.WindowBorder_C"))

(event `Player System Ready`
  (params (InSystemContext :type "SystemContext Object Reference"))
  (bind _returnvalue (`GameplayStatics.GetPlayerController` 0))
  ;[1 1 1] Set the current system context.
  (bind _output_get (set `self.My System` InSystemContext))
  (bind _returnvalue_2 (`SystemContext.GetDesktop` _output_get))
  ;[1 1 1] show desktop
  (`UserWidget.AddToViewport` _returnvalue_2 0)
  ;[1 1 1] Possess ourselves.
  (`Controller.Possess` _returnvalue self)
  (`WidgetBlueprintLibrary.SetInputMode_GameAndUIEx` _returnvalue _returnvalue_2 "DoNotLock" false)
  (add `PeacenetWorldStateActor.GameQuitRequested` (`SystemContext.GetPeacenet` _output_get) (delegate `Game Quit Requested`)))

(event `self.ReceiveUnpossessed`
  (params (OldController :type "Controller Object Reference"))
  ;[1 1 1] Remove the desktop from the screen.
  (`Widget.RemoveFromParent` (`SystemContext.GetDesktop` (`self.My System`)))
  ;[1 1 1] Spawn in the game splash screen.
  (bind _asplayer_controller (cast `PlayerController` OldController))
  (bind _returnvalue (`|SpawnActorFromClass` "/Game/Blueprints/Pawns/MenuPawn.MenuPawn_C" (`KismetMathLibrary.MakeTransform` (0.0 0.0 0.0)) "Undefined" "OverrideRootScale" null null))
  (`Controller.Possess` _asplayer_controller _returnvalue)
  ;[1 1 1] Destroy Peacegate actors forcing the game to save
  (`self.K2_DestroyActor` (`self.Peacenet`))
  (`self.K2_DestroyActor`))

(event `InputAction|Open Terminal`
  (params (Key :type "Key Structure"))
  (bind _returnvalue (`SystemContext.GetDesktop` (`self.My System`)))
  ;[1 1 1] Open a terminal as the current user of the desktop when the Open Terminal input action is released.
  (:`Released`
    (if (`DesktopWidget.IsSessionActive` _returnvalue)
      (`DesktopWidget.OpenProgram` _returnvalue "terminal"))))

(event `InputAction|Switch Text Mode`
  (params (Key :type "Key Structure"))
  (bind _returnvalue (`SystemContext.GetDesktop` (`self.My System`)))
  ;[1 1 1] Toggle text mode when the text mode input action is released.
  (:`Released`
    (if (`DesktopWidget.IsInTextMode` _returnvalue)
      (`DesktopWidget.DeactivateTextMode` _returnvalue)
      (else
        (`DesktopWidget.ActivateTextMode` _returnvalue)))))

(event `Game Quit Requested`
  ;[1 1 1] Unpossess the player's current pawn (us.)
  (`Controller.UnPossess` (`GameplayStatics.GetPlayerController` 0)))

(fn `UserConstructionScript`)